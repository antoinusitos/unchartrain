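; BP_CanonBall is a cannonball actor that damages destructible crates and trains it overlaps.
; Overlap handling runs only on the server, casting the other actor to BP_DestructibleCrates first, then BP_Train.
; Crates receive the Damage value, while the train's TakeDamage is called with no amount.
; The ball destroys itself after either hit and ignores all other actors.
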(event `self.ReceiveActorBeginOverlap`
  (params (OtherActor :type "Actor Object Reference"))
  (if (`KismetSystemLibrary.IsServer`)
    (`|ExecutionSequence`
      (:`then_0`
        (bind _asbp_destructible_crates (cast `/Game/UncharTrain/Blueprints/BP_DestructibleCrates` OtherActor)
          (:`then`
            (`/Game/UncharTrain/Blueprints/BP_DestructibleCrates.TakeDamage` _asbp_destructible_crates (`self.Damage`))
            (`self.K2_DestroyActor`))
          (:`CastFailed`
            (bind _asbp_train (cast `/Game/UncharTrain/Blueprints/BP_Train` OtherActor))
            (`UCT_Train.TakeDamage` _asbp_train)
            (`self.K2_DestroyActor`)))))))

(fn `UserConstructionScript`)