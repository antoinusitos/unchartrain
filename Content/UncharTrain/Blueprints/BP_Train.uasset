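; BP_Train is the train actor, with little active Blueprint logic beyond boost visual feedback.
; When the boost value changes, it feeds the ratio of BoostValue to BoostMax into a Niagara effect's boostFactor parameter.
; BeginPlay, AddTrainBreak and the construction script are empty.
; Disconnected leftover nodes would link stopper, booster and direction child actors back to the train, but never run.
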(event `self.ReceiveBeginPlay`)

(event `self.OnBoostValueChange`
  (`NiagaraComponent.SetVariableFloat` (`self.NewNiagaraSystem4`) "boostFactor" (/ (`self.BoostValue`) (`self.BoostMax`))))

(event `AddTrainBreak`)

(fn `UserConstructionScript`)