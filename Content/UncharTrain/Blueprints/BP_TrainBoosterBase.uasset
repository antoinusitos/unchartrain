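; BP_TrainBoosterBase is a base Blueprint for a train booster that displays a current value against a target on a widget.
; BeginPlay caches the WBP_Booster from its widget component.
; OnChangeDone linearly remaps the current value from input to output range onto one radial slider.
; It also sets a second slider's handle angles to a tolerance-wide band centered on the picked number, which is not remapped.
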(event `self.ReceiveBeginPlay`
  (bind _aswbp_booster (cast `/Game/UncharTrain/WBP/WBP_Booster` (`WidgetComponent.GetUserWidgetObject` (`self.Widget`))))
  (set `self.As WBP Booster` _aswbp_booster))

(event `self.OnChangeDone`
  (params (CurrentValue :type "Float (single-precision)") (PickedNumber :type Integer) (Tolerence :type "Float (single-precision)"))
  (bind _returnvalue (/ Tolerence 2.0))
  (bind _as_wbp_booster (`self.As WBP Booster`))
  (bind _targetradialslider (`/Game/UncharTrain/WBP/WBP_Booster.TargetRadialSlider` _as_wbp_booster))
  (`/Engine/EditorBlueprintResources/StandardMacros.IsValid` (`self.As WBP Booster`)
    (:`Is Valid`
      (`RadialSlider.SetValue` (`/Game/UncharTrain/WBP/WBP_Booster.CurrentRadialSlider` _as_wbp_booster) (+ (`self.OutputStart`) (* (/ (- (`self.OutputEnd`) (`self.OutputStart`)) (- (`self.InputEnd`) (`self.InputStart`))) (- CurrentValue (`self.InputStart`)))))
      (`RadialSlider.SetSliderHandleStartAngle` _targetradialslider (- PickedNumber _returnvalue))
      (`RadialSlider.SetSliderHandleEndAngle` _targetradialslider (+ PickedNumber _returnvalue)))))

(fn `UserConstructionScript`)